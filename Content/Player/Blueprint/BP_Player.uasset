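; BP_Player is the player-controlled pawn, handling basic movement and look input.
; BeginPlay limits vertical look by setting the camera manager's minimum and maximum view pitch.
; Move axes feed movement input along forward and right vectors derived from the controller's desired rotation.
; Look axes drive controller pitch and yaw, scaled by separate mouse sensitivity variables.
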(event EventBeginPlay
  (bind _returnvalue (Game|GetPlayerCameraManager 0))
  (|CallParentFunction)
  (Variables|/Script/Engine.PlayerCameraManager|SetViewPitchMin _returnvalue -65.0)
  (Variables|/Script/Engine.PlayerCameraManager|SetViewPitchMax _returnvalue 35.0))

(event Collision|EventActorBeginOverlap
  (params (OtherActor :type Actor%20Object%20Reference))
  (|CallParentFunction OtherActor) ; This node is disabled and will not be called.\nDrag off pins to build functionality.
)

(event EventTick
  (params (DeltaSeconds :type Float%20%28single-precision%29))
  (|CallParentFunction DeltaSeconds) ; This node is disabled and will not be called.\nDrag off pins to build functionality.
)

(event Input|AxisEvents|InputAxisMoveForward
  (params (AxisValue :type Float%20%28single-precision%29))
  (Pawn|Input|AddMovementInput (Math|Vector|GetForwardVector (Pawn|GetDesiredRotation (Pawn|GetController))) AxisValue false))

(event Input|AxisEvents|InputAxisMoveRight
  (params (AxisValue :type Float%20%28single-precision%29))
  (Pawn|Input|AddMovementInput (Math|Vector|GetRightVector (Pawn|GetDesiredRotation (Pawn|GetController))) AxisValue false))

(event Input|AxisEvents|InputAxisLookUp
  (params (AxisValue :type Float%20%28single-precision%29))
  (Pawn|Input|AddControllerPitchInput (* AxisValue (Variables|Default|GetMouseSensiY))))

(event Input|AxisEvents|InputAxisLookRight
  (params (AxisValue :type Float%20%28single-precision%29))
  (Pawn|Input|AddControllerYawInput (* AxisValue (Variables|Default|GetMouseSensiX))))

(fn ConstructionScript
  (|CallParentFunction))